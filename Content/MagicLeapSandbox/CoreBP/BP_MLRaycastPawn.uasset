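; Magic Leap sandbox pawn that continuously raycasts from the player's view and marks hit points with cubes.
; A looping timer started on BeginPlay sends Raycast component requests along the camera's forward vector several times a second.
; The asynchronous result delegate spawns a short-lived BP_Cube at each returned hit point, without checking the hit state.
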(event `self.ReceiveBeginPlay`
  (`KismetSystemLibrary.K2_SetTimerDelegate` (delegate `RequestRaycast`) 0.1 true))

(event `RequestRaycast`
  (bind _returnvalue (`GameplayStatics.GetPlayerCameraManager` 0))
  (`RaycastComponent.RequestRaycast` (`self.Raycast`) (make `RaycastQueryParams` (`self.K2_GetActorLocation` _returnvalue) (`self.GetActorForwardVector` _returnvalue) (0.0 0.0 0.0) 1 1 1.0) (delegate `RaycastResult`)))

(event `RaycastResult`
  (params (HitResult :type "RaycastHitResult Structure"))
  (bind _returnvalue (`|SpawnActorFromClass` "/Game/MagicLeapSandbox/Blueprints/BP_Cube.BP_Cube_C" (`KismetMathLibrary.MakeTransform` (`.HitPoint` (break `RaycastHitResult` HitResult))) "Undefined" "OverrideRootScale" null null))
  (`self.SetLifeSpan` _returnvalue 2.0))

(fn `UserConstructionScript`)